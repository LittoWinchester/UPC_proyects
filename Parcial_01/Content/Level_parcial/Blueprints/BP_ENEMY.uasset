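; BP_ENEMY is an enemy actor that moves by a per-frame offset and periodically fires bullets.
; SetVelocity stores the offset that Tick applies without sweep or frame-time scaling.
; Shoot stores a Target and latches Range on, letting a looping half-second timer spawn BP_Bullet at the enemy with Target as its velocity.
; The 20percent helper multiplies and divides by the same variable and is not called here.
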(event Custom|shooting
  (if (Variables|Default|GetRange?)
    (Game|SpawnActorfromClass "/Game/Level_parcial/Blueprints/BP_Bullet.BP_Bullet_C" (Math|Transform|MakeTransform (Transformation|GetActorLocation) "0, 0, 0" "1.000000,1.000000,1.000000") "Undefined" "MultiplyWithRoot" 0 (Variables|Default|Gettarget) 0)))

(event EventBeginPlay
  (Utilities|Time|SetTimerbyEvent (delegate Custom|shooting) 0.5 true))

(event Collision|EventActorBeginOverlap
  (params (OtherActor :type Actor%20Object%20Reference)))

(event EventTick
  (params (DeltaSeconds :type Float%20%28single-precision%29))
  (Transformation|AddActorLocalOffset (Variables|Default|GetMovement) false false))

(fn ConstructionScript)

(fn SetVelocity
  (params (Velocity :type Vector))
  (Variables|Default|SetMovement Velocity))

(fn 20percent
  (params (Inital :type Vector))
  (return (/ (* Inital (Variables|Default|GetX20)) (Variables|Default|GetX20))))

(fn Shoot
  (params (target :type Vector))
  (Variables|Default|Settarget target)
  (Variables|Default|SetRange? true))