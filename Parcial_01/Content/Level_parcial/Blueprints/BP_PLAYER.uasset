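; BP_PLAYER is a player actor that moves on its own by adding its Direction vector as an unswept local offset every tick.
; SetDirectionPlayer sets that vector from an input value.
; A looping timer started at BeginPlay runs an attack check that, while the under-attack flag is true, waits briefly, multiplies Direction by X2 and prints a speed-increase debug message.
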(event Custom|is%20atack?
  (if (Variables|Default|GetUnderAtatack)
    (Utilities|FlowControl|Delay 1.0)
    (Variables|Props|SetDirection (* (Variables|Default|Getx2) (Variables|Props|GetDirection)))
    (Development|PrintString "AUMENTE VELOCIDAD" true true "(R=1.000000,G=0.000000,B=0.180027,A=1.000000)" 5.0)))

(event EventBeginPlay
  (Utilities|Time|SetTimerbyEvent (delegate Custom|is%20atack?) 2.0 true))

(event Collision|EventActorBeginOverlap
  (params (OtherActor :type Actor%20Object%20Reference)))

(event EventTick
  (params (DeltaSeconds :type Float%20%28single-precision%29))
  (Transformation|AddActorLocalOffset (Variables|Props|GetDirection) false false))

(fn ConstructionScript)

(fn SetDirectionPlayer
  (params (Vector :type Vector))
  (Variables|Props|SetDirection Vector))