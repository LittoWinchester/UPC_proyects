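; BP_Archer is an archer actor that teleport-free moves to its stored initial position on BeginPlay and can fire BP_Arrow projectiles.
; Shoot spawns an arrow at the archer's location, passing the target vector as its velocity.
; The range-gated, delayed shooting logic is disconnected, so nothing in the file fires.
; CloserTarget, unused here, returns the larger of two values despite its name.
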(event EventBeginPlay
  (Transformation|SetActorLocation (Variables|Props|GetInitialPos) false false))

(event Collision|EventActorBeginOverlap
  (params (OtherActor :type Actor%20Object%20Reference)))

(event EventTick
  (params (DeltaSeconds :type Float%20%28single-precision%29)))

(fn ConstructionScript)

(fn Shoot
  (params (Target :type Vector))
  (Game|SpawnActorfromClass "/Game/Blueprints/BP_Arrow.BP_Arrow_C" (Math|Transform|MakeTransform (Transformation|GetActorLocation) "0, 0, 0" "1.000000,1.000000,1.000000") "Undefined" "MultiplyWithRoot" 0 Target 0))

(fn CloserTarget
  (params (Target1 :type Float%20%28double-precision%29) (target%202 :type Float%20%28double-precision%29))
  (if (> Target1 target%202)
    (return Target1)
    (else
      (return target%202))))